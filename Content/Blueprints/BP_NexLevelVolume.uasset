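; BP_NexLevelVolume is a trigger volume that checks whether the player has cleared the crystals needed to pass.
; On overlap by the player, it finds BP_Crystal actors sharing the volume's first tag, so each volume can track its own crystal group.
; It prints a pass message when none remain, or the remaining count otherwise.
; Feedback is print-only; no level transition is implemented here.
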(event Collision|EventActorBeginOverlap
  (params (OtherActor :type Actor%20Object%20Reference))
  (Utilities|IsPlayer OtherActor
    (:IsPlayer
      (bind _outactors (Actor|GetAllActorsOfClasswithTag "/Game/Blueprints/BP_Crystal.BP_Crystal_C" (Utilities|Array|Get(acopy) (Variables|Actor|GetTags))))
      (if (Utilities|Array|IsEmpty _outactors)
        (Development|PrintString "YOU CAN PASS")
        (else
          (Development|PrintString (Utilities|String|Append (Utilities|String|ToString(Integer) (Utilities|Array|Length _outactors)) " Crystals Left")))))))

(fn ConstructionScript)