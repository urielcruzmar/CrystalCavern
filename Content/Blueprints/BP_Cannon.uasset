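; BP_Cannon is a self-firing cannon that repeatedly launches BP_Projectile actors from the moment play begins.
; Each cycle waits for FireRate, spawns a scaled projectile at ProjectileSpawnPoint, then plays CannonFireTimeline.
; The timeline animates the barrel's relative Y position, and its Cannon Fired event track loops back to the delay to start the next shot.
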(event EventBeginPlay
  (Utilities|FlowControl|Delay (Variables|CannonProperties|GetFireRate) :!label _label)
  (CallFunction|SpawnProjectile)
  (bind _cannon_barrel_location (Timeline|Cannon%20Fire%20Timeline PlayFromStart)
    (:Update
      (CallFunction|MoveCannonBarrel _cannon_barrel_location))
    (:Cannon%20Fired
      (goto _label))))

(fn ConstructionScript)

(fn SpawnProjectile
  (bind _projectile_spawn_point (Variables|Default|GetProjectile%20Spawn%20Point))
  (Game|SpawnActorfromClass "/Game/Blueprints/BP_Projectile.BP_Projectile_C" (Math|Transform|MakeTransform (Transformation|GetWorldLocation _projectile_spawn_point) (Transformation|GetWorldRotation _projectile_spawn_point) (Math|Conversions|ToVector(Float) (Variables|CannonProperties|GetProjectileScale))) "Undefined" "MultiplyWithRoot" 0 0))

(fn MoveCannonBarrel
  (params (Connon%20Barrel%20Y%20Location :type Float%20%28double-precision%29))
  (Transformation|SetRelativeLocation (Variables|Default|GetCannon_Barrel) (Math|Vector|MakeVector 0.0 Connon%20Barrel%20Y%20Location 0.0) false false))