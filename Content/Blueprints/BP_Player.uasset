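; BP_Player is the player actor, moved by rolling physics torque on its static mesh, with a level restart when it takes damage.
; Forward/back and left/right axis inputs apply mass-independent torque around world X and Y, scaled by an acceleration multiplier.
; The camera fades in on BeginPlay.
; Any damage runs RestartLevel, which uses DoOnce to fade out once, wait for the fade, then reopen the current level.
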(event EventBeginPlay
  ;[1 1 1] Start Camera Fade
  (CameraFades|StartCameraFade :self (Game|GetPlayerCameraManager 0) :FromAlpha 1.0 :Duration (Variables|Default|GetFadeDuration)))

(event Game|Damage|EventAnyDamage
  (params (Damage :type Float%20%28single-precision%29) (DamageType :type Damage%20Type%20Object%20Reference) (InstigatedBy :type Controller%20Object%20Reference) (DamageCauser :type Actor%20Object%20Reference))
  ;[1 1 1] Restart Level
  (Utilities|RestartLevel))

(event Input|AxisEvents|InputAxisForward/Backwards
  (params (AxisValue :type Float%20%28single-precision%29))
  ;[1 1 1] Movement
  (Class|PrimitiveComponent|AddTorqueinRadians (Variables|Default|GetStaticMesh) (Math|Vector|MakeVector (* AxisValue (Variables|Default|GetAcccel%20Multiplier)) 0.0 0.0) "None" true))

(event Input|AxisEvents|InputAxisLeftRight
  (params (AxisValue :type Float%20%28single-precision%29))
  ;[1 1 1] Movement
  (Class|PrimitiveComponent|AddTorqueinRadians (Variables|Default|GetStaticMesh) (Math|Vector|MakeVector 0.0 (* AxisValue (Variables|Default|GetAcccel%20Multiplier)) 0.0) "None" true))

(fn ConstructionScript)